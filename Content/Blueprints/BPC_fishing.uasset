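; Fishing component that generates a random catch from a swappable fish data table and shows it on the ship controller's HUD.
; CatchFish scales the fish count by net area, density and random variation, then tallies quantity, total weight and largest weight per species.
; RandomFIsh takes the first row whose Rarity covers a random roll, falling back to row 1010.
; The cumulative-rarity weighted pick is disconnected.
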(event Custom|CatchFish
  (params (NetArea :type Float%20%28double-precision%29))
  (Utilities|Map|Clear (Variables|Default|GetCoughtFish))
  ;[1 1 1] Random ammount Fish
  (for _index (range 0 (Math|Float|Round (|((a*b)*c) (/ NetArea 1e+04) (Variables|Default|GetFishDensity) (Math|Random|RandomFloatinRange 0.6 1.2))))
    (bind (_fishid _fishname _weight _value_per_pound _icon) (CallFunction|RandomFIsh))
    (bind _result (Math|Integer|IncrementInt (.quantity (Utilities|Struct|BreakCaughtFish_struct (.Value (Utilities|Map|Find (Variables|Default|GetCoughtFish) _fishid)))))
      (:%20%20
        (Utilities|Map|Add (Variables|Default|GetCoughtFish) _fishid (Utilities|Struct|MakeCaughtFish_struct (Utilities|String|SelectString (.Name (Utilities|Struct|BreakCaughtFish_struct (.Value (Utilities|Map|Find (Variables|Default|GetCoughtFish) _fishid)))) _fishname (.ReturnValue (Utilities|Map|Find (Variables|Default|GetCoughtFish) _fishid))) (+ (.WeightTotal (Utilities|Struct|BreakCaughtFish_struct (.Value (Utilities|Map|Find (Variables|Default|GetCoughtFish) _fishid)))) _weight) _value_per_pound _result (Math|Float|SelectFloat (.MaxWeight (Utilities|Struct|BreakCaughtFish_struct (.Value (Utilities|Map|Find (Variables|Default|GetCoughtFish) _fishid)))) _weight (> (.MaxWeight (Utilities|Struct|BreakCaughtFish_struct (.Value (Utilities|Map|Find (Variables|Default|GetCoughtFish) _fishid)))) _weight)) _icon)))))
  (bind _asbp_ship_controls (Utilities|Casting|CastToBP_Ship_controls (Game|GetPlayerController 0)))
  (Default|DisplayCaughtFIhs (Variables|/Game/Blueprints/Player/BP_Ship_controls.BP_Ship_controls_C|GetHUd_Ref _asbp_ship_controls)))

(event Custom|UpdateFishTable
  (params (FishData :type Data%20Table%20Object%20Reference))
  (Variables|Default|SetFishData FishData))

(event EventBeginPlay
  ;[1 1 1] add tabel dat
)

(event Input|KeyboardEvents|DebugKey1
  (params (Key :type Key%20Structure :default "None") (ActionValue :type Input%20Action%20Value%20Structure))
  ;[1 1 1] Test catch
)

(fn GetDataforRandomFish
  (params (InFishData :type Data%20Table%20Object%20Reference))
  (Utilities|Map|Clear (Variables|Default|GetFishRaityData))
  (bind _outrownames (DataTable|GetDataTableRowNames InFishData))
  (for _array_element _outrownames
    (bind _returnvalue (Utilities|GetDataTableRow InFishData _array_element)
      (:then
        (Utilities|Map|Add (Variables|Default|GetFishRaityData) _array_element (.Rarity (Utilities|Struct|BreakFishData_struct _returnvalue))))))
  (bind _values (Utilities|Map|Values (Variables|Default|GetFishRaityData)))
  (for _array_element_2 _values
    (Variables|Default|SetAccumulatedRarity (+ (Variables|Default|GetAccumulatedRarity) _array_element_2))))

(fn RandomFIsh
  (LocalVariables|SetRadndomNum (Math|Random|RandomFloatinRange 0.0 1.0))
  (bind _outrownames (DataTable|GetDataTableRowNames (Variables|Default|GetFishData)))
  (for _array_element _outrownames
    (bind _returnvalue (Utilities|GetDataTableRow (Variables|Default|GetFishData) _array_element)
      (:then
        (if (<= (LocalVariables|GetRadndomNum) (.Rarity (Utilities|Struct|BreakFishData_struct _returnvalue)))
          (return _array_element (.Name (Utilities|Struct|BreakFishData_struct _returnvalue)) (CallFunction|RoundtoTwoDecimals (Math|Random|RandomFloatinRange (.minWeight (Utilities|Struct|BreakFishData_struct _returnvalue)) (.MaxWeight (Utilities|Struct|BreakFishData_struct _returnvalue)))) (.ValuePerPound (Utilities|Struct|BreakFishData_struct _returnvalue)) (.Icon (Utilities|Struct|BreakFishData_struct _returnvalue)))))))
  (bind _returnvalue_2 (Utilities|GetDataTableRow (Variables|Default|GetFishData) "1010")
    (:then
      (return "1010" (.Name (Utilities|Struct|BreakFishData_struct _returnvalue_2)) (CallFunction|RoundtoTwoDecimals (Math|Random|RandomFloatinRange (.minWeight (Utilities|Struct|BreakFishData_struct _returnvalue_2)) (.MaxWeight (Utilities|Struct|BreakFishData_struct _returnvalue_2)))) (.ValuePerPound (Utilities|Struct|BreakFishData_struct _returnvalue_2)) (.Icon (Utilities|Struct|BreakFishData_struct _returnvalue_2))))
    (:RowNotFound
      (Development|PrintString "hole in net"))))

(fn RoundtoTwoDecimals
  (params (A :type Float%20%28double-precision%29))
  (return (/ (Math|Conversions|ToFloat(Integer) (Math|Float|Round (* A 1e+02))) 1e+02)))