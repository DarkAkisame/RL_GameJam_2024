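; Player ship pawn that steers with physics torque, moves by interpolated forward velocity, and lays a net of buoys.
; Drop Net spawns a start buoy; Tick then adds net buoys at distance intervals while the MaxNetLength budget lasts.
; Returning near the start drops a final buoy and ends dropping.
; CalculateArea estimates the enclosed area from the ordered buoys with a trapezoid (shoelace-style) sum; look input is unwired.
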(event Custom|CheckCloseToStart
  ;[1 1 1] This checks to see if the player is done dropping net points
  (if (CallFunction|IsClosetoStart)
    (Variables|Default|SetDropping false)
    (CallFunction|DropNetPoint)))

(event Custom|DropNetPoint
  ;[1 1 1] Spawns the Net Point and adds it to the array - the array is in order of dropped
  (bind _returnvalue (Game|SpawnActorfromClass "/Game/Mesh/BP_NetBuoy.BP_NetBuoy_C" (Math|Transform|MakeTransform (Transformation|GetActorLocation) "0, 0, 0" "1.000000,1.000000,1.000000") "AlwaysSpawn" "MultiplyWithRoot" 0 0))
  (Utilities|Array|Add (Variables|Default|GetNetPointArray) _returnvalue))

(event Input|EnhancedActionEvents|EnhancedInputActionIA_Trun_Right
  (params (ActionValue :type Float%20%28double-precision%29) (ElapsedSeconds :type Float%20%28double-precision%29) (TriggeredSeconds :type Float%20%28double-precision%29) (InputAction :type Input%20Action%20Object%20Reference :default "/Game/Blueprints/Player/Inputs/Actions/IA_Trun_Right.IA_Trun_Right"))
  (Class|PrimitiveComponent|AddTorqueinDegrees (Variables|Default|GetStaticMesh) (Math|Vector|MakeVector 0.0 0.0 (* ActionValue 1e+02)) "None" true))

(event Input|EnhancedActionEvents|EnhancedInputActionIA_Move_Forward
  (params (ActionValue :type Float%20%28double-precision%29) (ElapsedSeconds :type Float%20%28double-precision%29) (TriggeredSeconds :type Float%20%28double-precision%29) (InputAction :type Input%20Action%20Object%20Reference :default "/Game/Blueprints/Player/Inputs/Actions/IA_Move_Forward.IA_Move_Forward"))
  (bind _returnvalue (+ ActionValue 1.0))
  (bind _staticmesh (Variables|Default|GetStaticMesh))
  (bind _returnvalue_2 (/ _returnvalue 2.0))
  (if (not (Math|Float|NearlyEqual(Float) _returnvalue_2 0.0 1e-06))
    (Variables|Default|SetThrust (Math|Interpolation|FInterpTo (Variables|Default|GetThrust) (Math|Float|Lerp 0.0 (Variables|Default|GetMaxThrust) _returnvalue_2) (Utilities|Time|GetWorldDeltaSeconds) 0.4))
    (Physics|SetPhysicsLinearVelocity _staticmesh (* (Math|Vector|GetForwardVector _staticmesh) (Variables|Default|GetThrust)) false "None")))

(event Input|EnhancedActionEvents|EnhancedInputActionIA_look
  (params (ActionValue :type Vector%202D%20Structure) (ElapsedSeconds :type Float%20%28double-precision%29) (TriggeredSeconds :type Float%20%28double-precision%29) (InputAction :type Input%20Action%20Object%20Reference :default "/Game/Blueprints/Player/Inputs/Actions/IA_look.IA_look")))

(event Input|EnhancedActionEvents|EnhancedInputActionIA_Drop_Net
  (params (ActionValue :type Boolean) (ElapsedSeconds :type Float%20%28double-precision%29) (TriggeredSeconds :type Float%20%28double-precision%29) (InputAction :type Input%20Action%20Object%20Reference :default "/Game/Blueprints/Player/Inputs/Actions/IA_Drop_Net.IA_Drop_Net"))
  (if (not (Variables|Default|GetDropping))
    (bind _output_get (Variables|Default|SetStartDropPoint (Transformation|GetActorLocation)))
    (Game|SpawnActorfromClass "/Game/Mesh/BP_StartBuoy.BP_StartBuoy_C" (Math|Conversions|ToTransform(Vector) _output_get) "Undefined" "MultiplyWithRoot" 0 0)
    (Variables|Default|SetLastDropPoint _output_get)
    (Utilities|Array|Clear (Variables|Default|GetNetPointArray))
    (if true
      (Variables|Default|SetDropping true)
      (else
        (Variables|Default|SetDropping false)))))

(event Collision|EventActorBeginOverlap
  (params (OtherActor :type Actor%20Object%20Reference)))

(event EventTick
  (params (DeltaSeconds :type Float%20%28single-precision%29))
  ;[1 1 1] On frame, if dropping, drop a new net point every DropAtMoveDistance
  (if (Variables|Default|GetDropping)
    (CallFunction|CheckClosetoStart)
    (if (and (> (Math|Float|Absolute(Float) (Math|Vector|Distance(Vector) (Transformation|GetActorLocation) (Variables|Default|GetLastDropPoint))) (Variables|Default|GetDrop%20at%20Move%20Distance)) (> (Variables|Default|GetMaxNetLength) 0))
      (bind _output_get (Variables|Default|SetMaxNetLength (- (Variables|Default|GetMaxNetLength) 1)))
      (CallFunction|DropNetPoint)
      (Variables|Default|SetLastDropPoint (Transformation|GetActorLocation))
      (Development|PrintString (Utilities|String|ToString(Integer) _output_get)))))

(fn ConstructionScript)

(fn IsClosetoStart
  (return (and (< (Math|Float|Absolute(Float) (Math|Vector|Distance(Vector) (Variables|Default|GetStartDropPoint) (Transformation|GetActorLocation))) (Variables|Default|GetDrop%20at%20Move%20Distance)) (Utilities|Operators|NotEqual(!=) (Variables|Default|GetLastDropPoint) (Variables|Default|GetStartDropPoint) 0.0))))

(fn CalculateArea
  (bind _netpointarray (Variables|Default|GetNetPointArray))
  (bind _returnvalue (Utilities|Array|Length _netpointarray))
  (bind _returnvalue_2 (- _returnvalue 1))
  (if (or (Variables|Default|GetDropping) (<= (Utilities|Array|Length (Variables|Default|GetNetPointArray)) 0))
    (return 0.0)
    (else
      (for _index (range 1 _returnvalue_2)
        (LocalVariables|SetArea (+ (LocalVariables|GetArea) (/ (|(((y+yi1)*(xi1-x))/2.000000) (.x (Transformation|GetActorLocation (Utilities|Array|Get(acopy) (Variables|Default|GetNetPointArray) _index))) (.y (Transformation|GetActorLocation (Utilities|Array|Get(acopy) (Variables|Default|GetNetPointArray) _index))) (.y (Transformation|GetActorLocation (Utilities|Array|Get(acopy) (Variables|Default|GetNetPointArray) (Math|Integer|%(Integer) (+ _index 1) _returnvalue_2)))) (.x (Transformation|GetActorLocation (Utilities|Array|Get(acopy) (Variables|Default|GetNetPointArray) (Math|Integer|%(Integer) (+ _index 1) _returnvalue_2))))) 2.0))))
      (return (Math|Float|Absolute(Float) (LocalVariables|GetArea))))))