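; Shop trigger volume that lets the player open the shop while their ship is inside it.
; A BP_Player_Ship entering the box enables the area's input, and leaving calls DisableInput on the player controller itself.
; The IA_shop action tells the HUD referenced by BP_Ship_controls to display the shop.
; The construction script sizes the box from VolumeSize.
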(event OnComponentBeginOverlap(Box)
  (params (OverlappedComponent :type Primitive%20Component%20Object%20Reference) (OtherActor :type Actor%20Object%20Reference) (OtherComp :type Primitive%20Component%20Object%20Reference) (OtherBodyIndex :type Integer) (bFromSweep :type Boolean) (SweepResult :type Hit%20Result%20Structure%20%28by%20ref%29))
  (Utilities|Casting|CastToBP_Player_Ship OtherActor)
  (Input|EnableInput (Game|GetPlayerController 0)))

(event OnComponentEndOverlap(Box)
  (params (OverlappedComponent :type Primitive%20Component%20Object%20Reference) (OtherActor :type Actor%20Object%20Reference) (OtherComp :type Primitive%20Component%20Object%20Reference) (OtherBodyIndex :type Integer))
  (Utilities|Casting|CastToBP_Player_Ship OtherActor)
  (Input|DisableInput (Game|GetPlayerController 0) 0))

(event Input|EnhancedActionEvents|EnhancedInputActionIA_shop
  (params (ActionValue :type Boolean) (ElapsedSeconds :type Float%20%28double-precision%29) (TriggeredSeconds :type Float%20%28double-precision%29) (InputAction :type Input%20Action%20Object%20Reference :default "/Game/Blueprints/Player/Inputs/Actions/IA_shop.IA_shop"))
  (:Started
    (bind _asbp_ship_controls (Utilities|Casting|CastToBP_Ship_controls (Game|GetPlayerController 0)))
    (Default|DIsplayShop (Variables|/Game/Blueprints/Player/BP_Ship_controls.BP_Ship_controls_C|GetHUd_Ref _asbp_ship_controls))))

(fn ConstructionScript
  (Components|Box|SetBoxExtent (Variables|Default|GetBox) (Variables|Default|GetVolumeSize) true))