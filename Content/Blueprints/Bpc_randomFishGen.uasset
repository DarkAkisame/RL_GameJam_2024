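; Blueprint component that generates random fish catches from a data table and keeps a per-species tally of the haul.
; On BeginPlay it caches and sums each row's rarity for cumulative weighted picks.
; CatchFish scales the roll count by net area, density and random variation, then merges each fish's weight, quantity and largest size into the CoughtFish map.
; Debug keys trigger a test catch and print the inventory.
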(event Custom|CatchFish
  (params (NetArea :type Float%20%28double-precision%29))
  ;[1 1 1] Random ammount Fish
  (for _index (range 0 (Math|Float|Round (|((a*b)*c) (/ NetArea 1e+02) (Variables|Default|GetFishDensity) (Math|Random|RandomFloatinRange 0.6 1.2))))
    (bind (_weight _value_per_pound _fishid _fishname) (CallFunction|RandomFIsh))
    (bind _result (Math|Integer|IncrementInt (.quantity (Utilities|Struct|BreakCaughtFish_struct (.Value (Utilities|Map|Find (Variables|Default|GetCoughtFish) _fishid)))))
      (:%20%20
        (Utilities|Map|Add (Variables|Default|GetCoughtFish) _fishid (Utilities|Struct|MakeCaughtFish_struct (Utilities|String|SelectString (.Name (Utilities|Struct|BreakCaughtFish_struct (.Value (Utilities|Map|Find (Variables|Default|GetCoughtFish) _fishid)))) _fishname (.ReturnValue (Utilities|Map|Find (Variables|Default|GetCoughtFish) _fishid))) (+ (.WeightTotal (Utilities|Struct|BreakCaughtFish_struct (.Value (Utilities|Map|Find (Variables|Default|GetCoughtFish) _fishid)))) _weight) _value_per_pound _result (Math|Float|SelectFloat (.MaxWeight (Utilities|Struct|BreakCaughtFish_struct (.Value (Utilities|Map|Find (Variables|Default|GetCoughtFish) _fishid)))) _weight (> (.MaxWeight (Utilities|Struct|BreakCaughtFish_struct (.Value (Utilities|Map|Find (Variables|Default|GetCoughtFish) _fishid)))) _weight)))))))
  (Utilities|Casting|CastToBP_Ship_controls (Game|GetPlayerController 0)))

(event EventBeginPlay
  ;[1 1 1] add tabel dat
  (CallFunction|GetDataforRandomFish (Variables|Default|GetFishData)))

(event Input|KeyboardEvents|1
  (params (Key :type Key%20Structure :default "None"))
  ;[1 1 1] Test catch
  (:Pressed
    (CallFunction|CatchFish 4e+04)))

(event Input|KeyboardEvents|3
  (params (Key :type Key%20Structure :default "None"))
  ;[1 1 1] Print inventory
  (:Pressed
    (bind _values (Utilities|Map|Values (Variables|Default|GetCoughtFish)))
    (for _array_element _values
      (Development|PrintString (Utilities|String|ToString(Text) (Utilities|Text|FormatText "You caught {quantity} {fishName}, with a total value of {Value}. The total weight is {weight} lbs, and the largest weighs {maxWeight} lbs" (.quantity (Utilities|Struct|BreakCaughtFish_struct _array_element)) (.Name (Utilities|Struct|BreakCaughtFish_struct _array_element)) (CallFunction|RoundtoTwoDecimals (* (.Value (Utilities|Struct|BreakCaughtFish_struct _array_element)) (.quantity (Utilities|Struct|BreakCaughtFish_struct _array_element)))) (CallFunction|RoundtoTwoDecimals (.WeightTotal (Utilities|Struct|BreakCaughtFish_struct _array_element))) (CallFunction|RoundtoTwoDecimals (.MaxWeight (Utilities|Struct|BreakCaughtFish_struct _array_element))))) true true "(R=0.000000,G=0.660000,B=1.000000,A=1.000000)" 1e+02))))

(fn GetDataforRandomFish
  (params (InFishData :type Data%20Table%20Object%20Reference))
  (bind _outrownames (DataTable|GetDataTableRowNames InFishData))
  (for _array_element _outrownames
    (bind _returnvalue (Utilities|GetDataTableRow InFishData _array_element)
      (:then
        (Utilities|Map|Add (Variables|Default|GetFishRaityData) _array_element (Utilities|Struct|BreakFishData_struct _returnvalue)))))
  (bind _values (Utilities|Map|Values (Variables|Default|GetFishRaityData)))
  (for _array_element_2 _values
    (Variables|Default|SetAccumulatedRarity (+ (Variables|Default|GetAccumulatedRarity) _array_element_2))))

(fn RandomFIsh
  (bind _fishraitydata (Variables|Default|GetFishRaityData))
  (LocalVariables|SetRandomID (Math|Random|RandomFloatinRange 0.0 (Variables|Default|GetAccumulatedRarity)))
  (bind _values (Utilities|Map|Values _fishraitydata))
  (bind (_array_element _array_index) (Utilities|Array|ForEachLoopwithBreak _values :!label _label)
    (:LoopBody
      (bind _output_get (LocalVariables|SetL_AccumulationRarity (+ (LocalVariables|GetL_AccumulationRarity) _array_element)))
      (if (> _output_get (LocalVariables|GetRandomID))
        (LocalVariables|SetFishIndex _array_index)
        (goto _label Break)))
    (:Completed
      (bind _keys (Utilities|Map|Keys _fishraitydata))
      (bind _returnvalue (Utilities|GetDataTableRow (Variables|Default|GetFishData) (Utilities|Array|Get(acopy) _keys (LocalVariables|GetFishIndex)))
        (:then
          (return (Math|Random|RandomFloatinRange (.minWeight (Utilities|Struct|BreakFishData_struct _returnvalue)) (.MaxWeight (Utilities|Struct|BreakFishData_struct _returnvalue))) (.ValuePerPound (Utilities|Struct|BreakFishData_struct _returnvalue)) (Utilities|Array|Get(acopy) _keys (LocalVariables|GetFishIndex)) (.Name (Utilities|Struct|BreakFishData_struct _returnvalue))))
        (:RowNotFound
          (Development|PrintString "fish not found"))))))

(fn RoundtoTwoDecimals
  (params (A :type Float%20%28double-precision%29))
  (return (/ (Math|Conversions|ToFloat(Integer) (Math|Float|Round (* A 1e+02))) 1e+02)))