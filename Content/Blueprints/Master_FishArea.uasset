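; Master fish area volume that changes which fish table the player ship's fishing uses inside a region.
; The construction script sizes the box from VolumeSize.
; When a BP_Player_Ship enters the box, its BPFishing receives AreaFishTable through UpdateFishTable.
; On exit it receives this area's DefualtFishTable, even if the ship is still inside another fish area.
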(event OnComponentBeginOverlap(Box)
  (params (OverlappedComponent :type Primitive%20Component%20Object%20Reference) (OtherActor :type Actor%20Object%20Reference) (OtherComp :type Primitive%20Component%20Object%20Reference) (OtherBodyIndex :type Integer) (bFromSweep :type Boolean) (SweepResult :type Hit%20Result%20Structure%20%28by%20ref%29))
  (bind _asbp_player_ship (Utilities|Casting|CastToBP_Player_Ship OtherActor))
  (Default|UpdateFishTable (Variables|/Game/Blueprints/Player/BP_Player_Ship.BP_Player_Ship_C|GetBP_Fishing _asbp_player_ship) (Variables|Default|GetAreaFishTable)))

(event OnComponentEndOverlap(Box)
  (params (OverlappedComponent :type Primitive%20Component%20Object%20Reference) (OtherActor :type Actor%20Object%20Reference) (OtherComp :type Primitive%20Component%20Object%20Reference) (OtherBodyIndex :type Integer))
  (bind _asbp_player_ship (Utilities|Casting|CastToBP_Player_Ship OtherActor))
  (Default|UpdateFishTable (Variables|/Game/Blueprints/Player/BP_Player_Ship.BP_Player_Ship_C|GetBP_Fishing _asbp_player_ship) (Variables|Default|GetDefualtFishTable)))

(fn ConstructionScript
  (Components|Box|SetBoxExtent (Variables|Default|GetBox) (Variables|Default|GetVolumeSize) true))