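; BP_PlayerBoat is a player boat Blueprint with an unfinished buoyancy test based on arrow components as sample points.
; Each Tick compares the first point's height to WaterLevel and, when it is below, sets that arrow's world location from the depth difference.
; The Boat component is never moved or pushed.
; Height checks for the other three points exist but are unconnected.
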(event EventBeginPlay)

(event Collision|EventActorBeginOverlap
  (params (OtherActor :type Actor%20Object%20Reference)))

(event EventTick
  (params (DeltaSeconds :type Float%20%28single-precision%29))
  (bind _arrow__buoyancypoint1_ (Variables|Default|GetArrow%20%28BuoyancyPoint1%29))
  (bind _returnvalue (Transformation|GetWorldLocation _arrow__buoyancypoint1_))
  (if (< (.z _returnvalue) (Variables|Default|GetWaterLevel))
    (Transformation|SetWorldLocation (Variables|Default|GetArrow%20%28BuoyancyPoint1%29) (- (Variables|Default|GetWaterLevel) (.z _returnvalue)) false false)))

(fn ConstructionScript)