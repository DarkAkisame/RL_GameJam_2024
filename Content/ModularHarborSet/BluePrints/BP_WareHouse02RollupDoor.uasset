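; Warehouse roll-up door Blueprint that opens and closes automatically on overlap with its trigger component.
; Any begin overlap plays Timeline_0 forward and end overlap reverses it, each spawning the roll-up door sound at world origin rather than at the door.
; Three vector tracks drive the relative locations of the three door meshes, with rotation reset to zero and scale to one on each update.
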(event OnComponentBeginOverlap(RollupDoorCillider)
  (params (OtherActor :type Actor%20Object%20Reference) (OtherComp :type Primitive%20Component%20Object%20Reference) (OtherBodyIndex :type Integer) (bFromSweep :type Boolean) (SweepResult :type Hit%20Result%20Structure%20%28by%20ref%29))
  (Audio|SpawnSoundatLocation "/Game/ModularHarborSet/Sounds/SC_RollupDoor.SC_RollupDoor" "0, 0, 0")
  (bind (_direction _rollupdoor _door2 _newtrack_10) (Timeline|Timeline_0 Play)
    (:Update
      (Transformation|SetRelativeTransform (Variables|Default|GetSM_RollupDoorPart01) (Math|Transform|MakeTransform _rollupdoor) false false)
      (Transformation|SetRelativeTransform (Variables|Default|GetSM_RollupDoorPart02) (Math|Transform|MakeTransform _door2) false false)
      (Transformation|SetRelativeTransform (Variables|Default|GetSM_RollupDoorPart03) (Math|Transform|MakeTransform _newtrack_10) false false))))

(event OnComponentEndOverlap(RollupDoorCillider)
  (params (OtherActor :type Actor%20Object%20Reference) (OtherComp :type Primitive%20Component%20Object%20Reference) (OtherBodyIndex :type Integer))
  (Audio|SpawnSoundatLocation "/Game/ModularHarborSet/Sounds/SC_RollupDoor.SC_RollupDoor" "0, 0, 0")
  (bind (_direction _rollupdoor _door2 _newtrack_10) (Timeline|Timeline_0 Reverse)
    (:Update
      (Transformation|SetRelativeTransform (Variables|Default|GetSM_RollupDoorPart01) (Math|Transform|MakeTransform _rollupdoor) false false)
      (Transformation|SetRelativeTransform (Variables|Default|GetSM_RollupDoorPart02) (Math|Transform|MakeTransform _door2) false false)
      (Transformation|SetRelativeTransform (Variables|Default|GetSM_RollupDoorPart03) (Math|Transform|MakeTransform _newtrack_10) false false))))

(fn ConstructionScript)